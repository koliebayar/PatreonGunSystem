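; BP_ShotgunMag is a shotgun magazine Blueprint that visually builds up its loaded rounds.
; AddRound increments SpawnedRounds and adds an instance to ISMRounds, offset along X by cartridge length so rounds line up in a row.
; Tick calls its parent and prints the round count as debug output, while the construction script only calls its parent.
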(event `self.ReceiveTick`
  (params (DeltaSeconds :type "Float (single-precision)"))
  (`parent.ReceiveTick` DeltaSeconds)
  (`KismetSystemLibrary.PrintString` (`KismetStringLibrary.Conv_IntToString` (`self.SpawnedRounds`))))

(fn `Add Round`
  (locals (CatridgeLength :type "Float (double-precision)" :default 6.9))
  (bind _output_get (set `self.SpawnedRounds` (+ (`self.SpawnedRounds`) 1)))
  (`InstancedStaticMeshComponent.AddInstance` (`self.ISM Rounds`) (`KismetMathLibrary.MakeTransform` (`KismetMathLibrary.MakeVector` (* (- _output_get 1) (`local.CatridgeLength`)))) false))

(fn `UserConstructionScript`
  (`parent.UserConstructionScript`))