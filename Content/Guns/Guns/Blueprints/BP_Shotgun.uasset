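; BP_Shotgun is a shotgun weapon Blueprint that equips itself with its own magazine actor when play begins.
; After the parent BeginPlay, it spawns a BP_ShotgunMag at the GunMesh "Magazine" socket, passing in magazine capacity and spawned round count.
; It stores the new actor as Magazine and snaps it to that socket.
; The construction script only calls the parent, and Tick and overlap events are disabled.
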(event `self.ReceiveBeginPlay`
  (`parent.ReceiveBeginPlay`)
  (bind _returnvalue (`|SpawnActorFromClass` "/Game/Guns/Guns/Shotgun/Blueprints/BP_ShotgunMag.BP_ShotgunMag_C" (`SceneComponent.GetSocketTransform` (`self.GunMesh`) "Magazine" "RTS_World") "Undefined" "MultiplyWithRoot" null (`self.Mag Max Cepacity`) (`self.Spawned Rounds`) null))
  (bind _output_get (set `self.Magazine` _returnvalue))
  (`self.K2_AttachToComponent` _output_get (`self.GunMesh`) "Magazine" "SnapToTarget" "SnapToTarget" "SnapToTarget" true))

(fn `UserConstructionScript`
  (`parent.UserConstructionScript`))