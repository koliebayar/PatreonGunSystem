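; VR hand grenade body that spawns a separately grabbable pin actor on its socket and explodes after being released with the pin removed.
; Grabbing the body enables pin collision and adds a per-hand input context disabling that trigger; pulling the pin starts looping haptics.
; Release detaches the physics lever and starts the detonation delay.
; Detonation plays effects, traces down for a scorch decal, fires a radial impulse and applies falloff damage.
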(event `self.ReceiveBeginPlay`
  (bind _curlgrabcomponent (`/Game/Guns/Granades/HandGranade/BP_GranadePin.CurlGrabComponent` (`self.GranadePin`)))
  (`self.SpawnGranadePin`)
  (add `/Game/VRTemplate/Blueprints/CurlGrabComponent.OnGrabbed` _curlgrabcomponent (delegate `OnGrabbed_Event`))
  (add `/Game/VRTemplate/Blueprints/CurlGrabComponent.OnDropped` _curlgrabcomponent (delegate `OnDropped_Event`)))

(event `OnDropped_Event`
  (`PrimitiveComponent.SetSimulatePhysics` (`/Game/Guns/Granades/HandGranade/BP_GranadePin.GranadePin` (`self.GranadePin`)) true))

(event `OnGrabbed_Event`
  (params (`Motion Controller` :type "MotionControllerComponent Object Reference"))
  (if (not (`self.PinIsTaken`))
    (set `self.PinIsTaken` true)
    (`PlayerController.PlayHapticEffect` (`GameplayStatics.GetPlayerController` 0) "/Game/VRTemplate/Haptics/GrabHapticEffect.GrabHapticEffect" (`/Game/VRTemplate/Blueprints/GrabComponent.GetHeldByHand` (`self.GrabComponent`)) 0.15 true)
    (`GameplayStatics.PlaySoundAtLocation` "/Game/Guns/Granades/Sounds/GranadePinRemove_Cue.GranadePinRemove_Cue" (`SceneComponent.K2_GetComponentLocation` (`/Game/Guns/Granades/HandGranade/BP_GranadePin.GranadePin` (`self.GranadePin`))) (struct) 1.0 1.0 0.0 null null null null)))

(event `self.GrabComponent.OnGrabbed`
  (params (`Motion Controller` :type "MotionControllerComponent Object Reference"))
  (`self.Motion Controller`
    (:`then`
      (`EnhancedInputSubsystemInterface.RemoveMappingContext` (pcsubsystem `EnhancedInputLocalPlayerSubsystem` (`GameplayStatics.GetPlayerController` 0)) (select `bool` (`|EnumEquality` (`/Game/VRTemplate/Blueprints/GrabComponent.GetHeldByHand` (`self.GrabComponent`)) "Right") :`false` "/Game/VRTemplate/Input/IMC_DisableTriggerButtonRight.IMC_DisableTriggerButtonRight" :`true` "/Game/VRTemplate/Input/IMC_DisableTriggerButtonLeft.IMC_DisableTriggerButtonLeft" :!type "InputMappingContext Object Reference") (struct)))
    (:`else`
      _))
  (set `self.Motion Controller` `Motion Controller`)
  (`self.EnableInput` (`GameplayStatics.GetPlayerController` 0))
  (`EnhancedInputSubsystemInterface.AddMappingContext` (pcsubsystem `EnhancedInputLocalPlayerSubsystem` (`GameplayStatics.GetPlayerController` 0)) (select `bool` (`|EnumEquality` (`/Game/VRTemplate/Blueprints/GrabComponent.GetHeldByHand` (`self.GrabComponent`)) "Left") :`false` "/Game/VRTemplate/Input/IMC_DisableTriggerButtonRight.IMC_DisableTriggerButtonRight" :`true` "/Game/VRTemplate/Input/IMC_DisableTriggerButtonLeft.IMC_DisableTriggerButtonLeft" :!type "InputMappingContext Object Reference") 1 (struct))
  (`self.SetActorEnableCollision` (`self.GranadePin`) true))

(event `OnComponentHit_Event`
  (params (HitComponent :type "PrimitiveComponent Object Reference") (OtherActor :type "Actor Object Reference") (OtherComp :type "PrimitiveComponent Object Reference") (NormalImpulse :type "Vector Structure") (Hit :type "HitResult Structure (by ref)"))
  (`KismetSystemLibrary.PrintString` "Hello" true true (struct :`R` 1.0 :`G` 0.01394 :`A` 1.0))
  (`/Engine/EditorBlueprintResources/StandardMacros.DoOnce` false
    (:`Completed`
      (`GameplayStatics.PlaySoundAtLocation` "/Game/Guns/Granades/Sounds/GranadeLeverDrop_Cue.GranadeLeverDrop_Cue" (`.Location` (`GameplayStatics.BreakHitResult` Hit)) (struct) 1.0 1.0 0.0 null null null null))))

(event `self.GrabComponent.OnDropped`
  (bind _granadelever (`self.GranadeLever`))
  (bind _pinistaken (`self.PinIsTaken`))
  (`self.SetActorEnableCollision` (`self.GranadePin`) _pinistaken)
  (if _pinistaken
    (`PlayerController.StopHapticEffect` (`GameplayStatics.GetPlayerController` 0) (`/Game/VRTemplate/Blueprints/GrabComponent.GetHeldByHand` (`self.GrabComponent`)))
    (`|ExecutionSequence`
      (:`then_0`
        (`KismetSystemLibrary.Delay` 0.35)
        (`SceneComponent.K2_DetachFromComponent` _granadelever "KeepWorld" "KeepWorld" "KeepWorld" true)
        (`PrimitiveComponent.SetSimulatePhysics` _granadelever true)
        (`Timeline|Timeline`
          (:`Update`
            (`SceneComponent.K2_AddLocalRotation` (`self.GranadeLever`) (struct :`Pitch` 10.0 :`Roll` 5.0) false false))
          (:`Finished`
            (`KismetSystemLibrary.PrintString` "Hello")
            (add `PrimitiveComponent.OnComponentHit` (`self.GranadeLever`) (delegate `OnComponentHit_Event`)))))
      (:`then_1`
        (`KismetSystemLibrary.Delay` (`self.DetonationTime`))
        (`self.ExplosionVFX&SFX`)
        (`self.Decals`)
        (`self.CheckIfSomeoneIsInRange`)
        (`|ExecutionSequence`
          (:`then_0`
            (`RadialForceComponent.FireImpulse` (`self.RadialForce`))
            (`KismetSystemLibrary.Delay` 0.2))
          (:`then_1`
            (`ActorComponent.K2_DestroyComponent` (`self.Flash`)))
          (:`then_2`
            (`self.K2_DestroyActor`))
          (:`then_3`
            (`self.RegisterDamage`))))
      (:`then_3`
        (`self.DisableInput` (`GameplayStatics.GetPlayerController` 0) :!label _label)
        (`EnhancedInputSubsystemInterface.RemoveMappingContext` (pcsubsystem `EnhancedInputLocalPlayerSubsystem` (`GameplayStatics.GetPlayerController` 0)) (select `bool` (`|EnumEquality` (`/Game/VRTemplate/Blueprints/GrabComponent.GetHeldByHand` (`self.GrabComponent`)) "Left") :`false` "/Game/VRTemplate/Input/IMC_DisableTriggerButtonRight.IMC_DisableTriggerButtonRight" :`true` "/Game/VRTemplate/Input/IMC_DisableTriggerButtonLeft.IMC_DisableTriggerButtonLeft" :!type "InputMappingContext Object Reference") (struct))))
    (else
      (goto _label))))

(fn `CheckIfSomeoneIsInRange`
  (if (> (`KismetArrayLibrary.Array_Length` (`PrimitiveComponent.GetOverlappingActors` (`self.DamageRadius`) "/Script/Engine.Pawn")) 0)
    (set `self.ExplodedWithingRangeOfAPlayer` true)))

(fn `Decals`
  (bind _returnvalue (`self.K2_GetActorLocation`))
  (bind (_outhit _returnvalue_2) (`KismetSystemLibrary.LineTraceSingleForObjects` _returnvalue (- _returnvalue (0.0 0.0 40.0)) (`|MakeArray` "ObjectTypeQuery1" :!type "EObjectTypeQuery Enum")))
  (if _returnvalue_2
    (bind (_bblockinghit _binitialoverlap _time _distance _location _impactpoint _normal _impactnormal) (`GameplayStatics.BreakHitResult` _outhit))
    (bind (_returnvalue_roll _returnvalue_pitch) (`KismetMathLibrary.BreakRotator` (`KismetMathLibrary.Conv_VectorToRotator` _impactnormal)))
    (bind _returnvalue_3 (`GameplayStatics.SpawnDecalAtLocation` "/Game/Guns/Granades/Materials/M_GranadeDecal.M_GranadeDecal" (* (`KismetMathLibrary.MakeVector` 1.0 130.0 130.0) (`KismetMathLibrary.RandomFloatInRange` 0.4 1.0)) _location (`KismetMathLibrary.MakeRotator` _returnvalue_roll _returnvalue_pitch (`KismetMathLibrary.RandomFloatInRange` 0.0 360.0)) 20.0))
    (`DecalComponent.SetFadeScreenSize` _returnvalue_3 0.01)
    (`DecalComponent.SetFadeOut` _returnvalue_3 17.0 10.0 false)))

(fn `ExplosionVFX&SFX`
  (bind _returnvalue (`SceneComponent.K2_GetComponentLocation` (`self.GranadeBody`)))
  (`GameplayStatics.PlaySoundAtLocation` (`self.ExplosionSound`) _returnvalue (struct) 1.0 1.0 0.0 null null null null)
  (`NiagaraFunctionLibrary.SpawnSystemAtLocation` (`self.ExplosionEffect`) _returnvalue)
  (bind _returnvalue_2 (`AddComponent|NODE_AddPointLightComponent-0` :`bManualAttachment` true :`RelativeTransform` (`self.GetTransform`)))
  (set `self.Flash` _returnvalue_2)
  (return))

(fn `RegisterDamage`
  (`GameplayStatics.ApplyRadialDamageWithFalloff` :`BaseDamage` (`self.Base Damage`) :`MinimumDamage` (`self.Minimum Damage`) :`Origin` (+ (`self.K2_GetActorLocation`) (0.0 0.0 20.0)) :`DamageInnerRadius` (`self.Damage Inner Radius`) :`DamageOuterRadius` (`self.Damage Outer Radius`) :`DamageFalloff` (`self.Damage Falloff`) :`DamageTypeClass` "/Script/Engine.DamageType" :`DamageCauser` self :`InstigatedByController` (`GameplayStatics.GetPlayerController` 0)))

(fn `SpawnGranadePin`
  (bind _returnvalue (`|SpawnActorFromClass` "/Game/Guns/Granades/HandGranade/BP_GranadePin.BP_GranadePin_C" (`self.GetTransform`) "Undefined" "MultiplyWithRoot" null null))
  (bind _output_get (set `self.GranadePin` _returnvalue))
  (`self.SetActorEnableCollision` _output_get false)
  (`self.K2_AttachToComponent` _output_get (`self.GranadeBody`) "Pin" "SnapToTarget" "SnapToTarget" "SnapToTarget" true))

(fn `UserConstructionScript`)